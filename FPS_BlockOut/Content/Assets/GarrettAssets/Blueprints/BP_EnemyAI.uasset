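; BP_EnemyAI is a simple enemy that chases the player and dies from a single projectile hit.
; A PawnSensing sighting triggers FollowPawn, which uses AI MoveTo toward player character 0, regardless of which pawn was seen.
; A hit from BP_FirstPersonProjectile destroys both the projectile and the enemy.
; No attack logic runs, as the only node that sets CanAttack is disconnected.
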(event OnSeePawn(PawnSensing)
  (params (Pawn :type Pawn%20Object%20Reference))
  (CallFunction|FollowPawn))

(event Custom|Follow%20Pawn
  (AI|AIMoveTo self "0, 0, 0" (Game|GetPlayerCharacter 0) 7e+01 false))

(event EventBeginPlay)

(event Collision|EventActorBeginOverlap
  (params (OtherActor :type Actor%20Object%20Reference)))

(event EventTick
  (params (DeltaSeconds :type Float%20%28single-precision%29)))

(event Collision|EventHit
  (params (MyComp :type Primitive%20Component%20Object%20Reference) (Other :type Actor%20Object%20Reference) (OtherComp :type Primitive%20Component%20Object%20Reference) (bSelfMoved :type Boolean) (HitLocation :type Vector :default "0, 0, 0") (HitNormal :type Vector :default "0, 0, 0") (NormalImpulse :type Vector :default "0, 0, 0") (Hit :type Hit%20Result%20Structure%20%28by%20ref%29))
  (Utilities|Casting|CastToBP_FirstPersonProjectile Other)
  (Actor|DestroyActor Other)
  (Actor|DestroyActor))

(fn ConstructionScript)